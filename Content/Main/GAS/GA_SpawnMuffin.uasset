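; Gameplay ability that spawns a unit (SpawnedUnit) at a player-confirmed target.
; On activation it adds a gameplay cue, then runs WaitTargetData with a start location built from the owner actor and the MainController's SpawnUnitLocation.
; Valid data commits the ability, adds another cue and feeds the SpawnActor task, which ends the ability on success.
; A failed commit or cancelled targeting cancels the ability.
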(event `self.K2_ActivateAbility`
  (bind (_locationtype _literaltransform _sourceactor _sourcecomponent _sourceability _sourcesocketname) (break `GameplayAbilityTargetingLocationInfo` (`self.MakeTargetLocationInfoFromOwnerActor`)))
  (bind _asgasbase_pawn (cast `GASBasePawn` (`self.GetAvatarActorFromActorInfo`)))
  (bind _output_get (set `self.As GASBase Pawn` _asgasbase_pawn))
  (bind _asmain_controller (cast `/Game/Main/MainController` (`Pawn.GetController` _output_get)))
  (set `self.As Main Controller` _asmain_controller)
  (`self.K2_AddGameplayCue` (struct))
  (bind (_asynctaskproxy _data) (`AbilityTask_WaitTargetData.WaitTargetData` "None" "UserConfirmed" (`self.TargetActorClass`) (make `GameplayAbilityTargetingLocationInfo` _locationtype (`KismetMathLibrary.MakeTransform` (`/Game/Main/MainController.SpawnUnitLocation` (`self.As Main Controller`)) (.rotation _literaltransform) (.scale _literaltransform)) _sourceactor _sourcecomponent _sourceability _sourcesocketname) (struct) null)
    (:`then`
      (set `self.Async Task` _asynctaskproxy))
    (:`ValidData`
      (bind _returnvalue (`self.K2_CommitAbility`))
      (if _returnvalue
        (`self.K2_AddGameplayCue` (struct))
        (`AbilityTask_SpawnActor.SpawnActor` _data (`self.SpawnedUnit`) null
          (:`Success`
            (`self.K2_EndAbility`)))
        (else
          (`self.K2_CancelAbility`))))
    (:`Cancelled`
      (`self.K2_CancelAbility`))))