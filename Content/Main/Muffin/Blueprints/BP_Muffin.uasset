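; BP_Muffin is an AI-controlled team unit that fights by eating and dies once its fullness reaches its maximum.
; DoAttack toggles a hitbox whose server-side overlaps lower an enemy muffin's max fullness or a building's fullness, while filling the attacker.
; Eaten projectiles both add fullness and shrink the maximum.
; StateComponent feeds a head-socket health widget, and death disables the hitbox, stops AI logic and sets a short lifespan.
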(event `self.ReceiveBeginPlay`
  (`self.UpdateFullnessWidget` (`self.StateComponent`)))

(event `self.Hitbox.OnComponentBeginOverlap`
  (params (OverlappedComponent :type "PrimitiveComponent Object Reference") (OtherActor :type "Actor Object Reference") (OtherComp :type "PrimitiveComponent Object Reference") (OtherBodyIndex :type Integer) (bFromSweep :type Boolean) (SweepResult :type "HitResult Structure (by ref)"))
  (bind _statecomponent (`self.StateComponent`))
  (bind _statecomponent_2 (`self.StateComponent`))
  (bind _statecomponent_3 (`self.StateComponent`))
  (bind _statecomponent_4 (`self.StateComponent`))
  (`/Engine/EditorBlueprintResources/ActorMacros.Switch Has Authority`
    (:`Authority`
      (bind _asbp_muffin (cast `/Game/Main/Muffin/Blueprints/BP_Muffin` OtherActor)
        (:`then`
          (if (`|EnumInequality` (`/Game/Main/Muffin/Blueprints/BP_Muffin.Team` _asbp_muffin) (`self.Team`))
            (`/Game/Main/Muffin/AI/StateComponent.RemoveMaxFullness` (`/Game/Main/Muffin/Blueprints/BP_Muffin.StateComponent` _asbp_muffin) (`StateComponent.Damage` (`self.StateComponent`)))
            (`/Game/Main/Muffin/AI/StateComponent.AddFullness` _statecomponent (/ (`StateComponent.Damage` _statecomponent) 2.0))
            (`self.UpdateFullnessWidget` (`self.StateComponent`))
            (`self.UpdateFullnessWidget` (`/Game/Main/Muffin/Blueprints/BP_Muffin.StateComponent` _asbp_muffin))
            (bind _statecomponent_5 (`/Game/Main/Muffin/Blueprints/BP_Muffin.StateComponent` _asbp_muffin))
            (if (not (not (>= (`StateComponent.Fullness` _statecomponent_5) (`StateComponent.MaxFullness` _statecomponent_5))))
              (`/Game/Main/Muffin/AI/StateComponent.Dead` _statecomponent_5)
              (`self.DestroyMuffin` _asbp_muffin))
            (if (>= (`StateComponent.Fullness` _statecomponent_3) (`StateComponent.MaxFullness` _statecomponent_3))
              (`/Game/Main/Muffin/AI/StateComponent.Dead` (`self.StateComponent`))
              (`self.DestroyMuffin`))))
        (:`CastFailed`
          (bind _asbp_base_building (cast `/Game/Main/Building/BP_BaseBuilding` OtherActor))
          (`/Game/Main/Muffin/AI/StateComponent.RemoveFullness` (`/Game/Main/Building/BP_BaseBuilding.StateComponent` _asbp_base_building) (`StateComponent.Damage` (`self.StateComponent`)))
          (`/Game/Main/Muffin/AI/StateComponent.AddFullness` _statecomponent_2 (`StateComponent.Damage` _statecomponent_2))
          (`self.UpdateFullnessWidget` (`self.StateComponent`))
          (`/Game/Main/Building/BP_BaseBuilding.UpdateFullnessWidget` _asbp_base_building (`/Game/Main/Building/BP_BaseBuilding.StateComponent` _asbp_base_building))
          (bind _statecomponent_6 (`/Game/Main/Building/BP_BaseBuilding.StateComponent` _asbp_base_building))
          (if (not (> (`StateComponent.Fullness` _statecomponent_6) 0.0))
            (`/Game/Main/Muffin/AI/StateComponent.Dead` _statecomponent_6)
            (`/Game/Main/Building/BP_BaseBuilding.DestroyBuilding` _asbp_base_building))
          (if (>= (`StateComponent.Fullness` _statecomponent_4) (`StateComponent.MaxFullness` _statecomponent_4))
            (`/Game/Main/Muffin/AI/StateComponent.Dead` (`self.StateComponent`))
            (`self.DestroyMuffin`)))))))

(event `EatProjectile(OnServer)`
  (params (Fulling :type "Float (double-precision)"))
  (bind _statecomponent (`self.StateComponent`))
  (`/Game/Main/Muffin/AI/StateComponent.AddFullness` (`self.StateComponent`) (/ Fulling 2.0))
  (`/Game/Main/Muffin/AI/StateComponent.RemoveMaxFullness` (`self.StateComponent`) (/ Fulling 2.0))
  (`self.UpdateFullnessWidget` (`self.StateComponent`))
  (if (>= (`StateComponent.Fullness` _statecomponent) (`StateComponent.MaxFullness` _statecomponent))
    (`/Game/Main/Muffin/AI/StateComponent.Dead` (`self.StateComponent`))
    (`self.DestroyMuffin`)))

(event `DestroyMuffin`
  (bind _returnvalue (`AIBlueprintHelperLibrary.GetAIController` self))
  (`PrimitiveComponent.SetCollisionEnabled` (`self.Hitbox`) "NoCollision")
  (if (`KismetSystemLibrary.IsValid` _returnvalue)
    (`BrainComponent.StopLogic` (`AIController.BrainComponent` _returnvalue) "")
    (`self.SetLifeSpan` 0.5)))

(event `self.StateComponent.OnFullnessChangedDelegate`
  (`self.UpdateFullnessWidget` (`self.StateComponent`)))

(fn `DoAttack`
  (params (IsAttacking :type Boolean))
  (bind _hitbox (`self.Hitbox`))
  (if IsAttacking
    (`PrimitiveComponent.SetCollisionEnabled` _hitbox "QueryOnly")
    (else
      (`PrimitiveComponent.SetCollisionEnabled` _hitbox "NoCollision")
      (set `StateComponent.MyUnitState` "Alive" (`self.StateComponent`)))))

(fn `UpdateFullnessWidget`
  (params (TargetStateComponent :type "/Game/Main/Muffin/AI/StateComponent Object Reference"))
  (bind _asw_unit_healt (cast `/Game/Main/UIX/W_UnitHealt` (`WidgetComponent.GetUserWidgetObject` (`self.Widget`))))
  (`/Game/Main/UIX/W_UnitHealt.Update HP` _asw_unit_healt (`StateComponent.Fullness` TargetStateComponent) (`StateComponent.MaxFullness` TargetStateComponent)))

(fn `UserConstructionScript`
  (`SceneComponent.K2_AttachToComponent` (`self.Widget`) (`self.Mesh`) "headSocket" "SnapToTarget" "SnapToTarget" "SnapToTarget" true))