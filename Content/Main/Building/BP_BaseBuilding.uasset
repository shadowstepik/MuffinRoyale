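; Base building actor that can fire team-owned projectiles and shows the fullness held by its StateComponent on a health-style widget.
; SpawnProjectile spawns a BP_BaseProjectile at an offset from the building, stores it and removes fullness equal to the component's Damage, so each shot drains the building.
; The W_UnitHealt widget refreshes on BeginPlay and whenever the fullness delegate fires.
; DestroyBuilding simply destroys the actor.
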(event `self.ReceiveBeginPlay`
  (`self.UpdateFullnessWidget` (`self.StateComponent`)))

(event `DestroyBuilding`
  (`self.K2_DestroyActor`))

(event `self.StateComponent.OnFullnessChangedDelegate`
  (`self.UpdateFullnessWidget` (`self.StateComponent`)))

(fn `SpawnProjectile`
  (bind (_returnvalue_location _returnvalue_rotation _returnvalue_scale) (`KismetMathLibrary.BreakTransform` (`self.GetTransform`)))
  (bind _statecomponent (`self.StateComponent`))
  (bind _returnvalue (`|SpawnActorFromClass` "/Game/Main/Building/BP_BaseProjectile.BP_BaseProjectile_C" (`KismetMathLibrary.MakeTransform` (+ (`self.ProjectileOffset`) _returnvalue_location) _returnvalue_rotation _returnvalue_scale) "Undefined" "OverrideRootScale" null (`self.Team`) null))
  (set `self.Projectile` _returnvalue)
  (`/Game/Main/Muffin/AI/StateComponent.RemoveFullness` _statecomponent (`StateComponent.Damage` _statecomponent)))

(fn `UpdateFullnessWidget`
  (params (TargetStateComponent :type "/Game/Main/Muffin/AI/StateComponent Object Reference"))
  (bind _asw_unit_healt (cast `/Game/Main/UIX/W_UnitHealt` (`WidgetComponent.GetUserWidgetObject` (`self.Widget`))))
  (`/Game/Main/UIX/W_UnitHealt.Update HP` _asw_unit_healt (`StateComponent.Fullness` TargetStateComponent) (`StateComponent.MaxFullness` TargetStateComponent)))

(fn `UserConstructionScript`)