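; BP_Castle is a castle building whose death ends the game.
; When its StateComponent fires OnDeadDelegate, it casts the current game mode to MainGameMode and calls GameEnd.
; Tick and the construction script only call their parent versions, and the BeginPlay and overlap events are disabled placeholders.
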(event `self.ReceiveTick`
  (params (DeltaSeconds :type "Float (single-precision)"))
  (`parent.ReceiveTick` DeltaSeconds))

(event `self.StateComponent.OnDeadDelegate`
  (bind _asmain_game_mode (cast `/Game/Main/MainGameMode` (`GameplayStatics.GetGameMode`)))
  (`/Game/Main/MainGameMode.GameEnd` _asmain_game_mode))

(fn `UserConstructionScript`
  (`parent.UserConstructionScript`))